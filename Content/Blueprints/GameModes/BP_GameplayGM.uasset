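; BP_GameplayGM is the Toon Tanks gameplay game mode, handling match start and end, tank respawns and logouts.
; Start and end events create the countdown, HUD and result widgets, passing in the start delay or win state.
; Respawn destroys any controlled pawn, then spawns and possesses the given tank class at a random PlayerStart.
; Swapped-in controllers are collected in an array, and logout has the game instance destroy that player's session.
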(event Custom|RespawnPlayer
  (params (PlayerController :type Player%20Controller%20Object%20Reference) (PlayerTank :type Pawn%20Class%20Reference))
  (bind _returnvalue (Pawn|GetControlledPawn PlayerController))
  ;[1 1 1] Spawn Player with Selected Tank
  (bind _outactors (Actor|GetAllActorsOfClass "/Script/Engine.PlayerStart"))
  (Variables|GameInfo|SetSpawnPoints _outactors)
  (Utilities|IsValid _returnvalue
    (:Is%20Valid
      (Actor|DestroyActor _returnvalue))
    (:Is%20Not%20Valid
      _))
  (bind _returnvalue_2 (Game|SpawnActorfromClass PlayerTank (Transformation|GetActorTransform (Utilities|Array|Get(acopy) (Variables|GameInfo|GetSpawnPoints) (Math|Random|RandomIntegerinRange 0 (- (Utilities|Array|Length (Variables|GameInfo|GetSpawnPoints)) 1)))) "Undefined" 0 0))
  (Pawn|Possess PlayerController _returnvalue_2))

(event EventOnSwapPlayerControllers
  (params (OldPC :type Player%20Controller%20Object%20Reference) (NewPC :type Player%20Controller%20Object%20Reference))
  ;[1 1 1] Fill Controllers Array
  (Utilities|Array|Add (Variables|GameInfo|GetAllPlayerControllers) NewPC))

(event EventOnLogout
  (params (ExitingController :type Controller%20Object%20Reference))
  ;[1 1 1] Destroy Session On Log Out
  (bind _asbp_gameplay_pc (Utilities|Casting|CastToBP_GameplayPC ExitingController))
  (Default|DestroySessionCaller (.AsBP%20Toon%20Tanks%20Game%20Instance (Utilities|Casting|CastToBP_ToonTanksGameInstance (Game|GetGameInstance))) _asbp_gameplay_pc))

(event EventGameStart
  ;[1 1 1] Game Start Delay & Game End Message
  (bind _returnvalue (UserInterface|CreateWidget "/Game/Blueprints/Widgets/WBP_Start.WBP_Start_C"))
  (Default|SetStartDelay _returnvalue (Variables|Default|GetStartDelay))
  (UserInterface|Viewport|AddtoViewport _returnvalue 0)
  (bind _returnvalue_2 (UserInterface|CreateWidget "/Game/Blueprints/Widgets/BP_Hud.BP_HUD_C"))
  (UserInterface|Viewport|AddtoViewport _returnvalue_2 0))

(event EventGameOver
  (params (PlayerWon :type Boolean))
  ;[1 1 1] Game Start Delay & Game End Message
  (bind _returnvalue (UserInterface|CreateWidget "/Game/Blueprints/Widgets/WBP_End.WBP_End_C"))
  (Default|SetPlayerWon _returnvalue PlayerWon)
  (UserInterface|Viewport|AddtoViewport _returnvalue 0))

(fn ConstructionScript)