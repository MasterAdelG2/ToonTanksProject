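; Lobby game mode for multiplayer Toon Tanks that manages joining, tank selection, kicking and travel to the chosen map.
; On login it registers each BP_LobbyPC, sets up its menu and possesses it with a base tank at a random PlayerStart.
; EveryoneUpdate rebuilds the player list and pushes it, with available tanks, to every controller.
; It also handles tank swaps, logout cleanup, ServerTravel by map ID and start/end widgets.
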(event Custom|SwapTank
  (params (PlayerController :type Player%20Controller%20Object%20Reference) (PawnClass :type Pawn%20Class%20Reference) (ChangedStatus :type Boolean))
  (bind _returnvalue (Pawn|GetControlledPawn PlayerController))
  (bind _spawnpoints (Variables|ServerSettings|GetSpawnPoints))
  ;[1 1 1] Swaps Tank
  (if (not ChangedStatus)
    (Utilities|IsValid _returnvalue
      (:Is%20Valid
        (Actor|DestroyActor _returnvalue))
      (:Is%20Not%20Valid
        _))
    (bind _returnvalue_2 (Game|SpawnActorfromClass PawnClass (Transformation|GetActorTransform (Utilities|Array|Get(acopy) _spawnpoints (Math|Random|RandomIntegerinRange 0 (- (Utilities|Array|Length _spawnpoints) 1)))) "Undefined" 0 0))
    (Pawn|Possess PlayerController _returnvalue_2)))

(event Custom|EveryoneUpdate
  (bind _allplayercontrollers (Variables|ServerSettings|GetAllPlayerControllers))
  ;[1 1 1] Update All Players Lobby Info When Called
  (bind _output_get (Variables|ServerSettings|SetCurrentPlayers (Utilities|Array|Length (Variables|ServerSettings|GetAllPlayerControllers))))
  (if (> _output_get 0)
    (Utilities|Array|Clear (Variables|ServerSettings|GetConnectedPlayers))
    (for _array_element _allplayercontrollers
      (bind _asbp_lobby_pc (Utilities|Casting|CastToBP_LobbyPC _array_element))
      (Utilities|Array|Add (Variables|ServerSettings|GetConnectedPlayers) (Variables|/Game/Blueprints/PlayerControllers/BP_LobbyPC.BP_LobbyPC_C|GetPlayerSettings _asbp_lobby_pc))
      (Default|UpdateNumberOfPlayers _asbp_lobby_pc (Variables|ServerSettings|GetCurrentPlayers) (Variables|ServerSettings|GetMax%20Players)))
    (for _array_element_2 _allplayercontrollers
      (bind _asbp_lobby_pc_2 (Utilities|Casting|CastToBP_LobbyPC _array_element_2))
      (Default|AddPlayerInfo _asbp_lobby_pc_2 (Variables|ServerSettings|GetConnectedPlayers))
      (Default|UpdateAvailableTanks _asbp_lobby_pc_2 (Variables|ServerSettings|GetAvailable%20Tanks))
      (CallFunction|AddtoKickList))
    (bind _array_element_3 (Utilities|Array|ForEachLoopwithBreak (Variables|ServerSettings|GetConnectedPlayers))
      (:LoopBody
        (bind _output_get_2 (Variables|ServerSettings|SetCanWeStart (select (== (Utilities|Struct|BreakPlayerInfo _array_element_3) "/Script/ToonTanks.PawnTank") false true)))
        (if (not _output_get_2)
          (CallFunction|CannotStartGame))))))

(event Custom|LaunchTheGame
  (bind _returnvalue (Game|GetPlayerController 0))
  ;[1 1 1] Launch Game Based On Map
  (switch int (Variables|ServerSettings|GetGMMap%20ID)
    (:0
      (Development|ExecuteConsoleCommand "ServerTravel /Game/Maps/Map_1" _returnvalue))
    (:1
      (Development|ExecuteConsoleCommand "ServerTravel /Game/Maps/Map_2" _returnvalue))))

(event Custom|RespawnPlayer
  (params (PlayerController :type Player%20Controller%20Object%20Reference))
  (bind _returnvalue (Pawn|GetControlledPawn PlayerController))
  (bind _spawnpoints (Variables|ServerSettings|GetSpawnPoints))
  ;[1 1 1] Spawn Character With Base Tank
  (Utilities|IsValid _returnvalue
    (:Is%20Valid
      (Actor|DestroyActor _returnvalue))
    (:Is%20Not%20Valid
      _))
  (bind _returnvalue_2 (Game|SpawnActorfromClass "/Game/Blueprints/Pawns/BP_PawnTank.BP_PawnTank_C" (Transformation|GetActorTransform (Utilities|Array|Get(acopy) _spawnpoints (Math|Random|RandomIntegerinRange 0 (- (Utilities|Array|Length _spawnpoints) 1)))) "Undefined" 0 0))
  (Pawn|Possess PlayerController _returnvalue_2)
  (CallFunction|EveryoneUpdate))

(event Custom|AddToKickList
  ;[1 1 1] Add Player To Kick List
  (bind _asbp_lobby_pc (Utilities|Casting|CastToBP_LobbyPC (Game|GetPlayerController 0)))
  (Utilities|IsValid (Variables|/Game/Blueprints/PlayerControllers/BP_LobbyPC.BP_LobbyPC_C|GetLobbyMenuWB _asbp_lobby_pc)
    (:Is%20Valid
      (if (Widget|IsVisible (Variables|/Game/Blueprints/Widgets/LobbyMenu.LobbyMenu_C|GetGameSettings (Variables|/Game/Blueprints/PlayerControllers/BP_LobbyPC.BP_LobbyPC_C|GetLobbyMenuWB _asbp_lobby_pc)))
        (Default|FillPlayersWindow (Variables|/Game/Blueprints/Widgets/LobbyMenu.LobbyMenu_C|GetGameSettings (Variables|/Game/Blueprints/PlayerControllers/BP_LobbyPC.BP_LobbyPC_C|GetLobbyMenuWB _asbp_lobby_pc)))))))

(event Custom|CannotStartGame
  ;[1 1 1] Update All Players Lobby Info When Called
  (Utilities|Array|ForEachLoopwithBreak (Variables|ServerSettings|GetConnectedPlayers)) ; enters at Break
)

(event Custom|ServerUpdateGameSettings
  (params (Map%20Image :type Texture%202D%20Object%20Reference) (MapName :type Text) (MapTime :type Text) (MapID :type Integer))
  ;[1 1 1] Server Made Changes & Tell Clients
  (Variables|ServerSettings|SetGMMapImage Map%20Image)
  (Variables|ServerSettings|SetGM_MapName MapName)
  (Variables|ServerSettings|SetGM_MapTime MapTime)
  (Variables|ServerSettings|SetGMMap%20ID MapID)
  (for _array_element (Variables|ServerSettings|GetAllPlayerControllers)
    (bind _asbp_lobby_pc (Utilities|Casting|CastToBP_LobbyPC _array_element))
    (Default|UpdateLobbySettings _asbp_lobby_pc (Variables|ServerSettings|GetGMMapImage) (Variables|ServerSettings|GetGM_MapName) (Variables|ServerSettings|GetGM_MapTime))))

(event Custom|YouHaveBeenKicked
  (params (PlayerID :type Integer))
  ;[1 1 1] Kicking
  (Default|Kicked (.AsBP%20Lobby%20PC (Utilities|Casting|CastToBP_LobbyPC (Utilities|Array|Get(acopy) (Variables|ServerSettings|GetAllPlayerControllers) PlayerID)))))

(event EventPostLogin
  (params (NewPlayer :type Player%20Controller%20Object%20Reference))
  ;[1 1 1] Initial Setup After Login
  (Networking|SwitchHasAuthority
    (:Authority
      (Utilities|Array|Add (Variables|ServerSettings|GetAllPlayerControllers) NewPlayer)
      (bind _outactors (Actor|GetAllActorsOfClass "/Script/Engine.PlayerStart"))
      (Variables|ServerSettings|SetSpawnPoints _outactors)
      (bind _asbp_toon_tanks_game_instance (Utilities|Casting|CastToBP_ToonTanksGameInstance (Game|GetGameInstance)))
      (Variables|ServerSettings|SetServer%20Name (Variables|/Game/Blueprints/BP_ToonTanksGameInstance.BP_ToonTanksGameInstance_C|GetServerName _asbp_toon_tanks_game_instance))
      (Variables|ServerSettings|SetMax%20Players (Variables|/Game/Blueprints/BP_ToonTanksGameInstance.BP_ToonTanksGameInstance_C|GetMaxPlayers _asbp_toon_tanks_game_instance))
      (bind _asbp_lobby_pc (Utilities|Casting|CastToBP_LobbyPC NewPlayer))
      (Default|InitialSetup _asbp_lobby_pc)
      (Default|SetupLobbyMenu _asbp_lobby_pc (Variables|ServerSettings|GetServer%20Name))
      (Default|UpdateLobbySettings _asbp_lobby_pc (Variables|ServerSettings|GetGMMapImage) (Variables|ServerSettings|GetGM_MapName) (Variables|ServerSettings|GetGM_MapTime))
      (CallFunction|RespawnPlayer NewPlayer))))

(event EventOnLogout
  (params (ExitingController :type Controller%20Object%20Reference))
  (bind _allplayercontrollers (Variables|ServerSettings|GetAllPlayerControllers))
  ;[1 1 1] LogOut Updates
  (Default|DestroySessionCaller (.AsBP%20Toon%20Tanks%20Game%20Instance (Utilities|Casting|CastToBP_ToonTanksGameInstance (Game|GetGameInstance))) (.AsBP%20Lobby%20PC (Utilities|Casting|CastToBP_LobbyPC ExitingController)))
  (bind (_array_element _array_index) (Utilities|Array|ForEachLoopwithBreak _allplayercontrollers :!label _label)
    (:LoopBody
      (if (== ExitingController _array_element)
        (goto _label Break)))
    (:Completed
      (bind _asbp_lobby_pc (Utilities|Casting|CastToBP_LobbyPC (Utilities|Array|Get(acopy) _allplayercontrollers _array_index)))
      (Utilities|Array|SetArrayElem (Variables|ServerSettings|GetAvailable%20Tanks) (Variables|/Game/Blueprints/PlayerControllers/BP_LobbyPC.BP_LobbyPC_C|GetSelectedTank _asbp_lobby_pc) false)
      (Utilities|Array|RemoveIndex (Variables|ServerSettings|GetAllPlayerControllers) _array_index)
      (Utilities|Array|RemoveIndex (Variables|ServerSettings|GetConnectedPlayers) _array_index)
      (CallFunction|EveryoneUpdate))))

(event EventGameStart
  (bind _returnvalue (UserInterface|CreateWidget "/Game/Blueprints/Widgets/WBP_Start.WBP_Start_C"))
  (Default|SetStartDelay _returnvalue (Variables|Default|GetStartDelay))
  (UserInterface|Viewport|AddtoViewport _returnvalue 0)
  (bind _returnvalue_2 (UserInterface|CreateWidget "/Game/Blueprints/Widgets/BP_Hud.BP_HUD_C"))
  (UserInterface|Viewport|AddtoViewport _returnvalue_2 0))

(event EventGameOver
  (params (PlayerWon :type Boolean))
  (bind _returnvalue (UserInterface|CreateWidget "/Game/Blueprints/Widgets/WBP_End.WBP_End_C"))
  (Default|SetPlayerWon _returnvalue PlayerWon)
  (UserInterface|Viewport|AddtoViewport _returnvalue 0))

(fn ConstructionScript)